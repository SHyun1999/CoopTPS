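; BP_GrenadeProjectile is a grenade actor that explodes on a short timer after BeginPlay.
; The explosion spawns a particle effect and applies falloff radial damage credited to the instigator's controller, with the inner radius set by a variable.
; It then destroys the actor and draws a debug sphere showing that inner radius.
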(event Custom|explode
  (bind _returnvalue (Transformation|GetActorLocation))
  (Effects|SpawnEmitteratLocation "/Game/WeaponEffects/Explosion/P_Explosion.P_Explosion" _returnvalue)
  (Class|GameplayStatics|ApplyRadialDamagewithFalloff 1e+02 5.0 _returnvalue (Variables|Default|GetDamage%20Inner%20Radius) 1e+01 0.1 0 0 self (Game|GetInstigatorController) "ECC_Visibility")
  (Actor|DestroyActor)
  (Rendering|Debug|DrawDebugSphere _returnvalue (Variables|Default|GetDamage%20Inner%20Radius) 12 "(R=1.000000,G=0.027276,B=0.000000,A=1.000000)" 1.0 2.0))

(event EventBeginPlay
  (Utilities|FlowControl|Delay 1.0)
  (CallFunction|Explode))

(fn ConstructionScript)